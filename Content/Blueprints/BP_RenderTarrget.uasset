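; BP_RenderTarrget is an actor that captures its own spinning Cube mesh component into a render target.
; The construction script assigns TextureTarget to the SceneCaptureComponent2D and adds the actor to its show-only list.
; It applies the Material override if valid; a valid Mesh triggers SetStaticMesh, though no mesh is passed to the call.
; Tick yaws the Cube at a constant, frame-rate-independent speed.
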(event `self.ReceiveBeginPlay`)

(event `self.ReceiveTick`
  (params (DeltaSeconds :type "Float (single-precision)"))
  (`SceneComponent.K2_AddRelativeRotation` (`self.Cube`) (`KismetMathLibrary.MakeRotator` 0.0 0.0 (* DeltaSeconds 30.0)) false false))

(fn `UserConstructionScript`
  (bind _scenecapturecomponent2d (`self.SceneCaptureComponent2D`))
  (bind _cube (`self.Cube`))
  (bind _material (`self.Material`))
  (`KismetArrayLibrary.Array_Add` (`SceneCaptureComponent.ShowOnlyActors` _scenecapturecomponent2d) self)
  (set `SceneCaptureComponent2D.TextureTarget` (`self.Texture Target`) _scenecapturecomponent2d)
  (`/Engine/EditorBlueprintResources/StandardMacros.IsValid` (`self.Mesh`)
    (:`Is Valid`
      (`StaticMeshComponent.SetStaticMesh` _cube null))
    (:`Is Not Valid`
      _))
  (`/Engine/EditorBlueprintResources/StandardMacros.IsValid` _material
    (:`Is Valid`
      (`PrimitiveComponent.SetMaterial` _cube 0 _material))))